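; Interaction component that finds the best nearby interactable for a pawn owner and stores it as the current target.
; While active on a pawn, a looping timer repeats sphere traces, ignoring each previous hit, to find actors with an active copy of this same component.
; Candidates need a clear visibility line trace and a narrow yaw from the owner's forward vector, and compete on combined distance and angle.
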(event `self.ReceiveBeginPlay`
  (`|ExecutionSequence`
    (:`then_0`
      (cast `Pawn` (`self.GetOwner`))
      (add `self.OnComponentActivated` (delegate `OnComponentActivated_Event_0`))
      (add `self.OnComponentDeactivated` (delegate `OnComponentDeactivated_Event_0`)))
    (:`then_1`
      (if (`self.ActiveOnStart`)
        (`self.Activate` false)
        (else
          (`self.Deactivate`))))))

(event `OnComponentActivated_Event_0` :!signature `self.OnComponentActivated`
  (params (Component :type "ActorComponent Object Reference") (bReset :type Boolean))
  (bind _returnvalue (`KismetSystemLibrary.K2_SetTimer` null "Timer_TraceInteractables" 0.075 true))
  (set `self.TraceHandle` _returnvalue))

(event `OnComponentDeactivated_Event_0` :!signature `self.OnComponentDeactivated`
  (params (Component :type "ActorComponent Object Reference"))
  (if (`KismetSystemLibrary.K2_IsValidTimerHandle` (`self.TraceHandle`))
    (`KismetSystemLibrary.K2_ClearAndInvalidateTimerHandle` (`self.TraceHandle`))))

(fn `Timer_TraceInteractables`
  (locals (L_CurrentTraceInore :type "Array of Actor Object Reference") (L_CurrentInteractionComp :type "/Game/SurvivalTPSTemp/Blueprints/Player/InteractionComponent/BP_SurvTPS_Interactions Object Reference") (L_OwnerLocation :type "Vector Structure" :default (0.0 0.0 0.0)) (L_NearestDistance :type "Float (double-precision)") (L_InteractionDirection :type "Vector Structure") (L_NearestRot :type "Float (double-precision)" :default 0.0) (L_CurrentNearestInteractComp :type "/Game/SurvivalTPSTemp/Blueprints/Player/InteractionComponent/BP_SurvTPS_Interactions Object Reference"))
  (bind _l_ownerlocation (`local.L_OwnerLocation`))
  (bind _l_ownerlocation_2 (`local.L_OwnerLocation`))
  (bind _l_nearestdistance (`local.L_NearestDistance`))
  (bind (_returnvalue_roll _returnvalue_pitch _returnvalue_yaw) (`KismetMathLibrary.BreakRotator` (`KismetMathLibrary.NormalizedDeltaRotator` (`KismetMathLibrary.Conv_VectorToRotator` (`local.L_InteractionDirection`)) (`KismetMathLibrary.Conv_VectorToRotator` (`Actor.GetActorForwardVector` (`self.GetOwner`))))))
  (bind _returnvalue (`KismetMathLibrary.Abs` _returnvalue_yaw))
  (bind _output_get (set `local.L_CurrentTraceInore` (`Actor.GetAttachedActors` (`self.GetOwner`) true false)))
  (`KismetArrayLibrary.Array_Add` _output_get (`self.GetOwner`))
  (set `local.L_CurrentNearestInteractComp` null)
  (set `local.L_OwnerLocation` (`Actor.K2_GetActorLocation` (`self.GetOwner`)))
  (for _ (range 1000)
    (bind (_outhit _returnvalue_2) (`KismetSystemLibrary.SphereTraceSingleForObjects` _l_ownerlocation (+ _l_ownerlocation (0.0 0.0 1.0)) 400.0 (`self.CollisionTypes`) false (`local.L_CurrentTraceInore`)))
    (if _returnvalue_2
      (bind (_bblockinghit _binitialoverlap _time _distance _location _impactpoint _normal _impactnormal _physmat _hitactor) (`GameplayStatics.BreakHitResult` _outhit))
      (`KismetArrayLibrary.Array_Add` (`local.L_CurrentTraceInore`) _hitactor)
      (bind _output_get_2 (set `local.L_CurrentInteractionComp` (`Actor.GetComponentByClass` _hitactor "BP_SurvTPS_Interactions_C")))
      (`/Engine/EditorBlueprintResources/StandardMacros.IsValid` _output_get_2
        (:`Is Valid`
          (if (`self.IsActive` (`local.L_CurrentInteractionComp`))
            (bind _output_get_3 (set `local.L_InteractionDirection` (`KismetMathLibrary.GetDirectionUnitVector` _l_ownerlocation_2 _impactpoint)))
            (bind _outhit_2 (`KismetSystemLibrary.LineTraceSingle` _l_ownerlocation_2 (+ _impactpoint (* _output_get_3 10.0)) "TraceTypeQuery1"))
            (bind (_bblockinghit_2 _binitialoverlap_2 _time_2 _distance_2 _location_2 _impactpoint_2 _normal_2 _impactnormal_2 _physmat_2 _hitactor_2) (`GameplayStatics.BreakHitResult` _outhit_2))
            (if (and (`KismetSystemLibrary.IsValid` _hitactor_2) (== _hitactor_2 _hitactor))
              (if (> _l_nearestdistance 0.0)
                (bind _returnvalue_3 (`KismetMathLibrary.Vector_Distance` (`local.L_OwnerLocation`) _impactpoint_2))
                (if (> (/ (+ (- _l_nearestdistance _returnvalue_3) (- (`local.L_NearestRot`) _returnvalue)) 2.0) 10.0)
                  (if (< _returnvalue 30.0) :!label _label
                    (set `local.L_NearestDistance` _returnvalue_3)
                    (set `local.L_NearestRot` _returnvalue)
                    (set `local.L_CurrentNearestInteractComp` (`local.L_CurrentInteractionComp`))))
                (else
                  (goto _label)))))))
      (else
        (break))))
  (`/Engine/EditorBlueprintResources/StandardMacros.IsValid` (`local.L_CurrentNearestInteractComp`)
    (:`Is Valid`
      (set `self.CurrentTargetInteractionComponent` (`local.L_CurrentNearestInteractComp`)))
    (:`Is Not Valid`
      (set `self.CurrentTargetInteractionComponent` null))))