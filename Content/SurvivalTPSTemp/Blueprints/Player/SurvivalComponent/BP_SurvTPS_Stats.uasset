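; Survival stats component for a Character, tracking health, food, water, energy and tiredness through clamped RepServ setter events.
; A looping timer sphere- and line-traces the ground for slope angle, then drains or recharges energy using fatigue curves, running and carried weight.
; Walking and jumping build tiredness, which lowers the restorable energy cap to no less than 25%.
; It also exposes slope-based input limits, jump checks, stat levels and an optional debug panel.
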(event `self.ReceiveBeginPlay`
  (bind _parentactor (`self.ParentActor`))
  (bind _ascharacter (cast `Character` (`self.GetOwner`)))
  (bind _output_get (set `self.ParentActor` _ascharacter))
  (`/Engine/EditorBlueprintResources/StandardMacros.IsValid` _output_get
    (:`Is Valid`
      (`self.RepServ_EnableTerrainTrace` true)
      (`|ExecutionSequence`
        (:`then_0`
          ;[1 1 1] Show debug if needed
          (if (and (`self.ShowDebugData`) (`Pawn.IsPlayerControlled` _parentactor) (`Pawn.IsLocallyControlled` _parentactor))
            (bind _returnvalue (`|CreateWidget` "/Game/SurvivalTPSTemp/Blueprints/Player/SurvivalComponent/UI/Debug/WBP_SurvTPS_DebugPanel.WBP_SurvTPS_DebugPanel_C"))
            (bind _output_get_2 (set `self.Runtime_DebugPanel` _returnvalue))
            (`/Game/SurvivalTPSTemp/Blueprints/Player/SurvivalComponent/UI/Debug/WBP_SurvTPS_DebugPanel.SetEnergyValue` _output_get_2 (`self.EnergyAmount`))
            (`UserWidget.AddToViewport` (`self.Runtime_DebugPanel`) 0)))
        (:`then_1`
          (`self.SetAllStatsToMax`))))))

(event `UpdateStatsOnServer`
  (params (`Stats(Server)` :type "/Game/SurvivalTPSTemp/Blueprints/Player/SurvivalComponent/Struct_SurvTPS_Stats_Server Structure"))
  (set `self.Stats(Server)` `Stats(Server)`))

(event `RepServ_EnableTerrainTrace`
  (params (Enable :type Boolean :default true))
  (bind _runtime_traceterrainhandler (`self.Runtime_TraceTerrainHandler`))
  ;[1 1 1] All
  (if Enable
    (bind _returnvalue (`KismetSystemLibrary.K2_SetTimer` null "Timer_TraceTerrain" (`self.TerrainTraceDeltaTime`) true))
    (set `self.Runtime_TraceTerrainHandler` _returnvalue)
    (elif (`KismetSystemLibrary.K2_IsValidTimerHandle` _runtime_traceterrainhandler)
      (`KismetSystemLibrary.K2_ClearAndInvalidateTimerHandle` _runtime_traceterrainhandler))))

(event `RepServ_MaxAll`
  ;[1 1 1] All
  (set `self.EnergyAmount` (`self.MaxEnergy`))
  (set `self.HealthAmount` (`self.HealthMax`))
  (set `self.FoodAmount` (`self.FoodMax`))
  (set `self.WaterAmount` (`self.WaterMax`)))

(event `RepServ_SetAllParameters`
  (params (EnergyAmount :type "Float (double-precision)") (HealthAmount :type "Float (double-precision)") (FoodAmount :type "Float (double-precision)") (WaterAmount :type "Float (double-precision)"))
  ;[1 1 1] All
  (set `self.EnergyAmount` (`KismetMathLibrary.FClamp` EnergyAmount 0.0 (`self.MaxEnergy`)))
  (set `self.HealthAmount` (`KismetMathLibrary.FClamp` HealthAmount 0.0 (`self.HealthMax`)))
  (set `self.FoodAmount` (`KismetMathLibrary.FClamp` FoodAmount 0.0 (`self.FoodMax`)))
  (set `self.WaterAmount` (`KismetMathLibrary.FClamp` WaterAmount 0.0 (`self.WaterMax`))))

(event `RepServ_SetWaterAmount`
  (params (NewWaterAmount :type "Float (double-precision)"))
  ;[0.1146 0.5857 1] Water
  (set `self.WaterAmount` (`KismetMathLibrary.FClamp` NewWaterAmount 0.0 (`self.WaterMax`))))

(event `RepServ_SetFoodAmount`
  (params (NewFoodAmount :type "Float (double-precision)"))
  ;[0.1615 0.0583 0.01254] Food
  (set `self.FoodAmount` (`KismetMathLibrary.FClamp` NewFoodAmount 0.0 (`self.FoodMax`))))

(event `RepServ_SetHealthAmount`
  (params (NewHealthAmount :type "Float (double-precision)"))
  ;[1 0 0] Health
  (set `self.FoodAmount` (`KismetMathLibrary.FClamp` NewHealthAmount 0.0 (`self.FoodMax`))))

(event `RepServ_SetEnergyAmount`
  (params (Amount :type "Float (double-precision)"))
  ;[1 0.9373 0.0697] Energy
  (set `self.EnergyAmount` (`KismetMathLibrary.FClamp` Amount 0.0 (`self.GetMaxEnergyBasedOnTiredness`))))

(event `RepServ_SetTiredness`
  (params (Amount :type "Float (double-precision)"))
  ;[0.2865 0.2865 0.2865] Tiredness
  (set `self.Tiredness` (`KismetMathLibrary.FClamp` Amount (`self.Tiredness`))))

(event `RepServ_ModifyWater`
  (params (Amount :type "Float (double-precision)"))
  ;[0.1146 0.5857 1] Water
  (`self.RepServ_SetWaterAmount` (+ (`self.WaterAmount`) Amount)))

(event `RepServ_ModifyFoodAmount`
  (params (Amount :type "Float (double-precision)"))
  ;[0.1615 0.0583 0.01254] Food
  (`self.RepServ_SetFoodAmount` (+ (`self.FoodMax`) Amount)))

(event `RepServ_ModifyHealthAmount`
  (params (Amount :type "Float (double-precision)"))
  ;[1 0 0] Health
  (`self.RepServ_SetHealthAmount` (+ (`self.HealthAmount`) Amount)))

(event `RepServ_ModifyTiredness`
  (params (Amount :type "Float (double-precision)"))
  ;[0.2865 0.2865 0.2865] Tiredness
  (`self.RepServ_SetTiredness` (+ (`self.Tiredness`) Amount)))

(event `RepServ_SubtractEnergy`
  (params (Amount :type "Float (double-precision)"))
  ;[1 0.9373 0.0697] Energy
  (`self.RepServ_SetEnergyAmount` (- (`self.EnergyAmount`) Amount)))

(fn `AddTiredness`
  (params (AmountToAdd :type "Float (double-precision)"))
  (`self.RepServ_ModifyTiredness` AmountToAdd))

(fn `CalculateWalkEnergyDrainAmount`
  (returns (ReturnValue :type "Float (double-precision)"))
  (bind _charactermovement (`Character.CharacterMovement` (`self.ParentActor`)))
  (return (* (`self.WalkingEnergyDrainFactor`) (`self.GetAngleFatigue`) (select `bool` (> (`CharacterMovementComponent.MaxWalkSpeed` _charactermovement) 300.0) :`false` 1.0 :`true` (`self.RunEnergyDrainMultiplier`)) (`KismetMathLibrary.VSize` (`KismetMathLibrary.Normal` (`MovementComponent.Velocity` _charactermovement))) (`self.GetWeightInfluence`))))

(fn `CanJump?`
  (returns (Value :type Boolean))
  (return (> (`self.EnergyAmount`) (`self.GetJumpEnergyCost`))))

(fn `GetAngleFatigue`
  (returns (ReturnValue :type "Float (single-precision)"))
  (bind _walkanglefatiguecurve (`self.WalkAngleFatigueCurve`))
  (`/Engine/EditorBlueprintResources/StandardMacros.IsValid` _walkanglefatiguecurve
    (:`Is Valid`
      (return (`CurveFloat.GetFloatValue` _walkanglefatiguecurve (`self.CurrentWalkingAngle`))))
    (:`Is Not Valid`
      (return 0.0))))

(fn `GetEnergyLevel`
  (returns (ReturnValue :type "Float (double-precision)"))
  (bind _maxenergy (`self.MaxEnergy`))
  (if (> _maxenergy 0.0)
    (return (`KismetMathLibrary.FMax` (/ (`self.EnergyAmount`) _maxenergy)))
    (else
      (return -1.0))))

(fn `GetFoodLevel`
  (returns (ReturnValue :type "Float (double-precision)"))
  (bind _foodmax (`self.FoodMax`))
  (if (> _foodmax 0.0)
    (return (`KismetMathLibrary.FMax` (/ (`self.FoodAmount`) _foodmax)))
    (else
      (return -1.0))))

(fn `GetHealthLevel`
  (returns (ReturnValue :type "Float (double-precision)"))
  (bind _healthmax (`self.HealthMax`))
  (if (> _healthmax 0.0)
    (return (`KismetMathLibrary.FMax` (/ (`self.HealthAmount`) _healthmax)))
    (else
      (return -1.0))))

(fn `GetInputLimit`
  (returns (InputLimit :type "Float (single-precision)"))
  (bind _walkingangleinputlimitcurve (`self.WalkingAngleInputLimitCurve`))
  (`/Engine/EditorBlueprintResources/StandardMacros.IsValid` _walkingangleinputlimitcurve
    (:`Is Valid`
      (return (`KismetMathLibrary.FClamp` (`CurveFloat.GetFloatValue` _walkingangleinputlimitcurve (`self.CurrentWalkingAngle`)))))
    (:`Is Not Valid`
      (return 0.0))))

(fn `GetJumpEnergyCost`
  (returns (ReturnValue :type "Float (double-precision)"))
  (return (`KismetMathLibrary.MultiplyMultiply_FloatFloat` (`self.JumpEnergyDrainFactor`) (`self.GetWeightInfluence`))))

(fn `GetMaxEnergyBasedOnTiredness`
  (returns (ReturnValue :type "Float (double-precision)"))
  (bind _maxenergy (`self.MaxEnergy`))
  (return (- _maxenergy (* (`KismetMathLibrary.FClamp` (`self.Tiredness`) 0.0 0.75) _maxenergy))))

(fn `GetWaterLevel`
  (returns (ReturnValue :type "Float (double-precision)"))
  (bind _watermax (`self.WaterMax`))
  (if (> _watermax 0.0)
    (return (`KismetMathLibrary.FMax` (/ (`self.WaterAmount`) _watermax)))
    (else
      (return -1.0))))

(fn `GetWeightInfluence`
  (returns (ReturnValue :type "Float (double-precision)"))
  (bind _weightloadinfluencecurve (`self.WeightLoadInfluenceCurve`))
  (`/Engine/EditorBlueprintResources/StandardMacros.IsValid` _weightloadinfluencecurve
    (:`Is Valid`
      (return (`CurveFloat.GetFloatValue` _weightloadinfluencecurve (`self.Runtime_CurrentWeightLoad`))))
    (:`Is Not Valid`
      (return 0.0))))

(fn `JumpEnergyDrain`
  (bind _returnvalue (`self.GetJumpEnergyCost`))
  (`self.SubtractEnergy` _returnvalue)
  (`self.AddTiredness` (* _returnvalue (`self.TirednessGlobalFactor`) (`self.JumpTirednessFactor`)))
  (return))

(fn `OnRep_ParentActor`
  (`/Engine/EditorBlueprintResources/StandardMacros.IsValid` (`self.ParentActor`)))

(fn `Set Food Amount`
  (params (NewFoodAmount :type "Float (double-precision)"))
  (`self.RepServ_SetFoodAmount` NewFoodAmount)
  (return))

(fn `Set Water Amount`
  (params (NewAmount :type "Float (double-precision)"))
  (`self.RepServ_SetWaterAmount` NewAmount)
  (return))

(fn `SetAllStatsToMax`
  (`self.RepServ_MaxAll`)
  (return))

(fn `SetEnergyAmount`
  (params (Amount :type "Float (double-precision)"))
  (`self.RepServ_SetEnergyAmount` Amount)
  (return))

(fn `SetHealthAmount`
  (params (NewHealthAmount :type "Float (double-precision)"))
  (`self.RepServ_SetHealthAmount` NewHealthAmount)
  (return))

(fn `SetTiredness`
  (params (Amount :type "Float (double-precision)"))
  (`self.RepServ_SetTiredness` Amount)
  (return))

(fn `SubtractEnergy`
  (params (`Amount(Subtract)` :type "Float (double-precision)"))
  ;[1 1 1] Set new Energy Value and update the widget
  (`self.RepServ_SubtractEnergy` `Amount(Subtract)`)
  (return))

(fn `Timer_ServerStatsUpdate`
  (bind (_stats_server__walkingangle _stats_server__energy _stats_server__tiredness) (break `/Game/SurvivalTPSTemp/Blueprints/Player/SurvivalComponent/Struct_SurvTPS_Stats_Server` (`self.Stats(Server)`)))
  (`|ExecutionSequence`
    (:`then_0`
      (if (and (or (!= _stats_server__walkingangle (`self.CurrentWalkingAngle`)) (!= _stats_server__energy (`self.EnergyAmount`)) (!= _stats_server__tiredness (`self.Tiredness`))) (`Pawn.IsLocallyControlled` (`self.ParentActor`)))
        (`self.UpdateStatsOnServer` (make `/Game/SurvivalTPSTemp/Blueprints/Player/SurvivalComponent/Struct_SurvTPS_Stats_Server` (`self.CurrentWalkingAngle`) (`self.EnergyAmount`) (`self.Tiredness`)))))))

(fn `Timer_TraceTerrain`
  (locals (L_ActorsToIgnore :type "Array of Actor Object Reference"))
  (bind _returnvalue (`self.CalculateWalkEnergyDrainAmount`))
  (bind _runtime_debugpanel (`self.Runtime_DebugPanel`))
  (bind _parentactor (`self.ParentActor`))
  (bind _parentactor_2 (`self.ParentActor`))
  (bind _returnvalue_2 (`Actor.K2_GetActorLocation` _parentactor_2))
  (bind _capsulecomponent (`Character.CapsuleComponent` _parentactor_2))
  (bind _velocity (`MovementComponent.Velocity` (`Character.CharacterMovement` _parentactor)))
  (bind _returnvalue_3 (* (`KismetMathLibrary.SelectFloat` _returnvalue (* (* (/ (* (`self.EnergyRechargeFactor`) 10.0) (`self.GetWeightInfluence`)) -1.0) (`KismetMathLibrary.MapRangeClamped` _returnvalue 0.0 (`self.EnergyDrain/RechargeLimit`) 1.0)) (> _returnvalue (`self.EnergyDrain/RechargeLimit`))) (`self.TerrainTraceDeltaTime`)))
  (if (`NavMovementComponent.IsFalling` (`Character.CharacterMovement` (`self.ParentActor`)))
    (set `self.CurrentWalkingAngle` 0.0)
    ;[1 1 1] Debug
    (if (`KismetSystemLibrary.IsValid` (`self.Runtime_DebugPanel`)) :!label _label
      (`/Game/SurvivalTPSTemp/Blueprints/Player/SurvivalComponent/UI/Debug/WBP_SurvTPS_DebugPanel.SetEnergyValue` _runtime_debugpanel (`self.EnergyAmount`))
      (`/Game/SurvivalTPSTemp/Blueprints/Player/SurvivalComponent/UI/Debug/WBP_SurvTPS_DebugPanel.SetEnergyConsumption` _runtime_debugpanel _returnvalue_3)
      (`/Game/SurvivalTPSTemp/Blueprints/Player/SurvivalComponent/UI/Debug/WBP_SurvTPS_DebugPanel.SetWalkAngleValue` _runtime_debugpanel (`self.CurrentWalkingAngle`))
      (`/Game/SurvivalTPSTemp/Blueprints/Player/SurvivalComponent/UI/Debug/WBP_SurvTPS_DebugPanel.SetInputLimit` _runtime_debugpanel (`self.GetInputLimit`))
      (`/Game/SurvivalTPSTemp/Blueprints/Player/SurvivalComponent/UI/Debug/WBP_SurvTPS_DebugPanel.SetWeightInfluence` _runtime_debugpanel (`self.GetWeightInfluence`))
      (`/Game/SurvivalTPSTemp/Blueprints/Player/SurvivalComponent/UI/Debug/WBP_SurvTPS_DebugPanel.SetTirednessValue` _runtime_debugpanel (`self.Tiredness`)))
    (else
      ;[1 1 1] Actors to ignore when tracing
      (bind _output_get (set `local.L_ActorsToIgnore` (`Actor.GetAttachedActors` (`self.ParentActor`) true false)))
      (`KismetArrayLibrary.Array_Add` _output_get (`self.ParentActor`))
      ;[1 1 1] Trace area under capsule
      (bind (_outhit _returnvalue_4) (`KismetSystemLibrary.SphereTraceSingleForObjects` (- _returnvalue_2 (`KismetMathLibrary.MakeVector` 0.0 0.0 (`CapsuleComponent.GetScaledCapsuleHalfHeight_WithoutHemisphere` _capsulecomponent))) (- _returnvalue_2 (`KismetMathLibrary.MakeVector` 0.0 0.0 (* (`CapsuleComponent.GetScaledCapsuleHalfHeight` _capsulecomponent) 1.2))) (* (`CapsuleComponent.GetScaledCapsuleRadius` _capsulecomponent) 0.5) (`self.WalkableObjectTypes`) false (`local.L_ActorsToIgnore`)))
      ;[1 1 1] If collision is found trace line for accurate normal
      (if _returnvalue_4
        (bind (_bblockinghit _binitialoverlap _time _distance _location _impactpoint) (`GameplayStatics.BreakHitResult` _outhit))
        (bind (_outhit_2 _returnvalue_5) (`KismetSystemLibrary.LineTraceSingleForObjects` (+ _impactpoint (0.0 0.0 50.0)) (- _impactpoint (0.0 0.0 50.0)) (`self.WalkableObjectTypes`) false (`local.L_ActorsToIgnore`)))
        (if _returnvalue_5
          (set `self.CurrentWalkingAngle` (/ (.pitch (`KismetMathLibrary.Conv_VectorToRotator` (`KismetMathLibrary.GetReflectionVector` (`KismetMathLibrary.SelectVector` (`Actor.GetActorForwardVector` _parentactor) (`KismetMathLibrary.Normal` _velocity) (== (`KismetMathLibrary.VSize` _velocity) 0.0)) (`.ImpactNormal` (`GameplayStatics.BreakHitResult` _outhit_2))))) 2)) ; Store current angle
          ;[1 1 1] Tiredness is constantly increasing by a fraction of the spent energy, multiplied by the WalingTirednessFactor
          (`self.AddTiredness` (* _returnvalue (`self.TirednessGlobalFactor`) (`self.WalkTirednessFactor`) (`self.TerrainTraceDeltaTime`)))
          (`self.SubtractEnergy` _returnvalue_3)
          (goto _label))))))

(fn `UseInputLimit`
  (params (Input :type "Float (double-precision)"))
  (returns (ReturnValue :type "Float (double-precision)"))
  (bind _inputlimit (`self.GetInputLimit`))
  (return (`KismetMathLibrary.FClamp` Input (* _inputlimit -1.0) _inputlimit)))