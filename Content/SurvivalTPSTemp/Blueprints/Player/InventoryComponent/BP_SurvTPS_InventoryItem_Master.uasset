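; Base inventory item actor for the survival TPS template, carrying item data and able to hold stored items as a container.
; Its construction script shows either the static mesh or an added skeletal mesh, based on the visual component type.
; Get/SetItemData convert between the actor and an inventory struct.
; Used storage volume is summed from stored items and sent through a server event, while the stored-items OnRep refreshes player 0's inventory UI.
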(event `RecalculateVolumeInUse`
  (set `self.Runtime_StorageVolumeUsed` 0.0)
  (for _array_element (`self.Runtime_StoredItems`)
    (set `self.Runtime_StorageVolumeUsed` (+ (`self.Runtime_StorageVolumeUsed`) (`.Volume_40_1972588B431ACEAE109F41A7DE4D9040` (break `/Game/SurvivalTPSTemp/Blueprints/Player/InventoryComponent/Struct_SurvTPS_InventoryObject` _array_element))))))

(event `self.ReceiveTick`
  (params (DeltaSeconds :type "Float (single-precision)")))

(event `self.ReceiveBeginPlay`
  (`|ExecutionSequence`
    (:`then_1`
      (`self.UpdateStorageVolumeUsed`))))

(event `RepServer_SetStorageVolumeUsed`
  (params (Runtime_StorageVolumeUsed :type "Float (double-precision)"))
  (set `self.Runtime_StorageVolumeUsed` Runtime_StorageVolumeUsed))

(fn `GetItemData`
  (returns (Struct_SurvTPS_InventoryObject :type "/Game/SurvivalTPSTemp/Blueprints/Player/InventoryComponent/Struct_SurvTPS_InventoryObject Structure"))
  (`self.UpdateStorageVolumeUsed`)
  (return (make `/Game/SurvivalTPSTemp/Blueprints/Player/InventoryComponent/Struct_SurvTPS_InventoryObject` self (`GameplayStatics.GetObjectClass` self) (`self.ItemName`) (`self.Icon`) (`self.CanBeStored`) (`self.Volume`) (`self.Weight`) (`self.StorageVolumeMax`) (`self.Runtime_StorageVolumeUsed`))))

(fn `OnRep_Runtime_StoredItems`
  (bind _returnvalue (`GameplayStatics.GetPlayerPawn` 0))
  (`/Engine/EditorBlueprintResources/StandardMacros.IsValid` _returnvalue
    (:`Is Valid`
      (`/Engine/EditorBlueprintResources/StandardMacros.IsValid` _returnvalue
        (:`Is Valid`
          (`/Game/SurvivalTPSTemp/Blueprints/Player/InventoryComponent/BP_SurvTPS_Inventory.UpdateInventoryUI` (`self.GetComponentByClass` _returnvalue "/Game/SurvivalTPSTemp/Blueprints/Player/InventoryComponent/BP_SurvTPS_Inventory.BP_SurvTPS_Inventory_C")))))))

(fn `SetItemData`
  (params (InData :type "/Game/SurvivalTPSTemp/Blueprints/Player/InventoryComponent/Struct_SurvTPS_InventoryObject Structure"))
  (bind (_itemreference _class _itemname _icon _canbestored _volume _weight _storagevolumemax _runtime_storagevolumeinuse) (break `/Game/SurvivalTPSTemp/Blueprints/Player/InventoryComponent/Struct_SurvTPS_InventoryObject` InData))
  (`|ExecutionSequence`
    (:`then_0`
      (set `self.ItemName` _itemname))
    (:`then_1`
      (set `self.Icon` _icon))
    (:`then_2`
      (set `self.CanBeStored` _canbestored))
    (:`then_3`
      (set `self.Volume` _volume))
    (:`then_4`
      (set `self.Weight` _weight))
    (:`then_6`
      (set `self.StorageVolumeMax` _storagevolumemax))
    (:`then_7`
      (set `self.Runtime_StorageVolumeUsed` _runtime_storagevolumeinuse))
    (:`then_8`
      (return))))

(fn `UpdateStorageVolumeUsed`
  (returns (NewVolume :type "Float (double-precision)"))
  (locals (L_TotalVolume :type "Float (double-precision)"))
  (bind _l_totalvolume (`local.L_TotalVolume`))
  (for _array_element (`self.Runtime_StoredItems`)
    (set `local.L_TotalVolume` (+ (`local.L_TotalVolume`) (`.Volume_40_1972588B431ACEAE109F41A7DE4D9040` (break `/Game/SurvivalTPSTemp/Blueprints/Player/InventoryComponent/Struct_SurvTPS_InventoryObject` _array_element)))))
  (`self.RepServer_SetStorageVolumeUsed` _l_totalvolume)
  (set `self.Runtime_StorageVolumeUsed` _l_totalvolume)
  (return _l_totalvolume))

(fn `UserConstructionScript`
  (bind _staticmesh (`self.StaticMesh`))
  (switch `/Game/SurvivalTPSTemp/Blueprints/Player/InventoryComponent/Enum_SurvTPS_VisualComponent` (`self.VisualComponentType`)
    (:`NewEnumerator0`
      (set `self.VisualComponent` _staticmesh)
      (`StaticMeshComponent.SetStaticMesh` _staticmesh (`self.VisualStaticMesh`))
      (`SceneComponent.SetVisibility` (`self.StaticMesh`) true true)
      (`PrimitiveComponent.SetCollisionEnabled` (`self.StaticMesh`) "QueryOnly"))
    (:`NewEnumerator1`
      (bind _returnvalue (`AddComponent|NODE_AddSkeletalMeshComponent-2` :`RelativeTransform` (`KismetMathLibrary.MakeTransform` (0.0 0.0 0.0))))
      (bind _output_get (set `self.VisualComponent` _returnvalue))
      (`SkinnedMeshComponent.SetSkinnedAssetAndUpdate` _returnvalue (`self.VisualSkeletalMesh`) true)
      (`SceneComponent.K2_SetRelativeTransform` _output_get (`SceneComponent.GetRelativeTransform` (`self.StaticMesh`)) false false)
      (`SceneComponent.SetVisibility` (`self.StaticMesh`) false true)
      (`PrimitiveComponent.SetCollisionEnabled` (`self.StaticMesh`) "NoCollision"))))