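; Base inventory equipment item that characters wear when equipped and that lies in the world when unequipped.
; Equipping attaches the actor and adds a skeletal mesh to the character, whose RepNotify assigns mesh and materials and follows the body via master pose.
; A multicast hides the world visual and disables its collision.
; Unequipping destroys the worn mesh, traces down and multicasts the restored visual onto the surface with random yaw.
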(event `self.ReceiveTick`
  (params (DeltaSeconds :type "Float (single-precision)"))
  (`parent.ReceiveTick` DeltaSeconds))

(event `Unequip_Multi`
  (params (NewLocation :type "Vector Structure") (NewRotation :type "Rotator Structure") (`Delta Rotation Z (Yaw)` :type "Float (single-precision)"))
  ;[1 1 1] Equi/Unequip multicast
  (`SceneComponent.SetVisibility` (`self.VisualComponent`) true false)
  (`PrimitiveComponent.SetCollisionEnabled` (`self.VisualComponent`) (`self.Runtime_DefaultCollisionEnabled`))
  (`self.K2_SetActorLocationAndRotation` NewLocation NewRotation)
  (`self.K2_AddActorLocalRotation` (`KismetMathLibrary.MakeRotator` 0.0 0.0 `Delta Rotation Z (Yaw)`)))

(event `Equip_Multi`
  ;[1 1 1] Equi/Unequip multicast
  (`SceneComponent.SetVisibility` (`self.VisualComponent`) false false)
  (`|ExecutionSequence`
    (:`then_0`
      (`/Engine/EditorBlueprintResources/StandardMacros.DoOnce` false
        (:`Completed`
          (set `self.Runtime_DefaultCollisionEnabled` (`PrimitiveComponent.GetCollisionEnabled` (`self.VisualComponent`))))))
    (:`then_1`
      (`PrimitiveComponent.SetCollisionEnabled` (`self.VisualComponent`) "NoCollision"))))

(fn `EquipItem`
  (params (Owner :type "Actor Object Reference"))
  (bind _asbp_surv_tps_character_master (cast `/Game/SurvivalTPSTemp/Blueprints/Player/BP_SurvTPS_CharacterMaster` Owner))
  (bind _output_get (set `self.Runtime_CurrentOwningCharacter` _asbp_surv_tps_character_master))
  (`self.K2_AttachToActor` _output_get "None" "SnapToTarget" "SnapToTarget" "SnapToTarget" false)
  (bind _returnvalue (`AddComponent|NODE_AddSkeletalMeshComponent-3` :`self` self :`RelativeTransform` (`SceneComponent.GetRelativeTransform` (`Character.Mesh` (`self.Runtime_CurrentOwningCharacter`)))))
  (bind _output_get_2 (set `self.SkeletalMeshOnCharacter` _returnvalue))
  (`SceneComponent.K2_AttachToComponent` _output_get_2 (`Character.Mesh` (`self.Runtime_CurrentOwningCharacter`)) "None" "SnapToTarget" "SnapToTarget" "SnapToTarget" false)
  (`self.SetOwner` (`self.Runtime_CurrentOwningCharacter`))
  (`self.Equip_Multi`)
  (return))

(fn `OnRep_SkeletalMeshOnCharacter`
  (bind _skeletalmeshoncharacter (`self.SkeletalMeshOnCharacter`))
  (`/Engine/EditorBlueprintResources/StandardMacros.IsValid` _skeletalmeshoncharacter
    (:`Is Valid`
      (`SkinnedMeshComponent.SetSkinnedAssetAndUpdate` _skeletalmeshoncharacter (`self.VisualSkeletalMesh`) true)
      (`SkinnedMeshComponent.SetLeaderPoseComponent` _skeletalmeshoncharacter (`Character.Mesh` (`self.Runtime_CurrentOwningCharacter`)) false)
      (for (_array_element _array_index) (`MeshComponent.GetMaterials` (`self.VisualComponent`))
        (`PrimitiveComponent.SetMaterial` (`self.SkeletalMeshOnCharacter`) _array_index _array_element))
      (return))))

(fn `UnequipItem`
  (bind _returnvalue (`self.K2_GetActorLocation`))
  (`self.K2_DetachFromActor` "KeepWorld" "KeepWorld" "KeepWorld")
  (`self.SetOwner` null)
  (`ActorComponent.K2_DestroyComponent` (`self.SkeletalMeshOnCharacter`))
  (bind (_outhit _returnvalue_2) (`KismetSystemLibrary.SphereTraceSingleForObjects` _returnvalue (- _returnvalue (0.0 0.0 1000.0)) 4.0 (`|MakeArray` "ObjectTypeQuery1" "ObjectTypeQuery2" :!type "EObjectTypeQuery Enum")))
  (if _returnvalue_2
    (bind (_bblockinghit _binitialoverlap _time _distance _location _impactpoint _normal _impactnormal) (`GameplayStatics.BreakHitResult` _outhit))
    (`self.Unequip_Multi` _impactpoint (`KismetMathLibrary.MakeRotFromZ` _impactnormal) (`KismetMathLibrary.RandomFloatInRange` 0.0 360.0))
    (return)
    (else
      (`self.Unequip_Multi` (`self.K2_GetActorLocation`))
      (return))))

(fn `UserConstructionScript`
  (`parent.UserConstructionScript`))