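; Master projectile Blueprint for the survival TPS template, simulating projectile flight with stepped traces on a looping timer.
; Each step advances along the forward vector by speed, adds growing weight-scaled gravity drop, and traces that segment.
; Exceeding maximum distance or a line-trace hit stops the timer; hits only print the actor's name.
; Sphere and box trace options are stubs without endpoints or hit handling.
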(event `self.ReceiveBeginPlay`
  (bind _returnvalue (`KismetSystemLibrary.K2_SetTimer` null "Timer_TraceProjectile" (`self.Runtime_DeltaTimeTrace`) true))
  (set `self.Runtime_TraceHandle` _returnvalue)
  (set `self.Runtime_LastProjectileLocation` (`self.K2_GetActorLocation`)))

(fn `Timer_TraceProjectile`
  (locals (L_InitialLocation :type "Vector Structure" :default (0.0 0.0 0.0)) (L_EndLocation :type "Vector Structure"))
  (bind _returnvalue (+ (`KismetMathLibrary.Vector_Distance` (`local.L_InitialLocation`) (`local.L_EndLocation`)) (`self.Runtime_DistanceTravelled`)))
  (bind _output_get (set `local.L_InitialLocation` (`self.Runtime_LastProjectileLocation`)))
  (bind _output_get_2 (set `self.Runtime_GravityOffset` (+ (`self.Runtime_GravityOffset`) (* (* (`self.Gravity`) (`self.Weight`)) (`self.Runtime_DeltaTimeTrace`)))))
  (set `local.L_EndLocation` (- (+ _output_get (* (`self.GetActorForwardVector`) (* (`self.Speed`) (`self.Runtime_DeltaTimeTrace`)))) (`KismetMathLibrary.MakeVector` 0.0 0.0 _output_get_2)))
  (if (> _returnvalue (`self.DistanceMax`))
    (`KismetSystemLibrary.K2_ClearAndInvalidateTimerHandle` (`self.Runtime_TraceHandle`))
    (else
      (set `self.Runtime_DistanceTravelled` _returnvalue)
      (set `self.Runtime_LastProjectileLocation` (`local.L_EndLocation`))
      (switch `/Game/SurvivalTPSTemp/Blueprints/Player/InventoryComponent/Weapons/Projectiles/Enum_SurvTPS_ProjectileTraceTypes` (`self.TraceType`)
        (:`NewEnumerator0`
          (bind (_outhit _returnvalue_2) (`KismetSystemLibrary.LineTraceSingle` :`Start` (`local.L_InitialLocation`) :`End` (`local.L_EndLocation`) :`TraceChannel` "TraceTypeQuery1" :`DrawDebugType` "ForDuration"))
          (if _returnvalue_2
            (`KismetSystemLibrary.K2_ClearAndInvalidateTimerHandle` (`self.Runtime_TraceHandle`))
            (`KismetSystemLibrary.PrintString` (`KismetSystemLibrary.GetDisplayName` (`.HitActor` (`GameplayStatics.BreakHitResult` _outhit))))))
        (:`NewEnumerator1`
          (`KismetSystemLibrary.SphereTraceSingle` (0.0 0.0 0.0) (0.0 0.0 0.0) 0.0 "TraceTypeQuery1"))
        (:`NewEnumerator2`
          (`KismetSystemLibrary.BoxTraceSingle` (0.0 0.0 0.0) (0.0 0.0 0.0) (0.0 0.0 0.0) (struct) "TraceTypeQuery1"))))))

(fn `UserConstructionScript`
  (`parent.UserConstructionScript`))