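; Gun weapon item for the survival TPS inventory, handling projectile fire and reloading for its owning character.
; On attack stop, a ready gun sends its muzzle socket transform to a replicated event that spends magazine ammo and spawns the projectile.
; Reload locks the gun and plays a montage via server and multicast events.
; Montage blend-out refills the magazine from inventory ammo typed by projectile class defaults, while interruption only restores readiness.
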(event `/Game/SurvivalTPSTemp/Blueprints/Player/InventoryComponent/Weapons/Master/BP_SurvTPS_InventoryItem_Weapon_Master.WInput_Attack_1`
  (params (`Action/Stop` :type Boolean))
  ;[1 1 1] Fire
  (`parent.WInput_Attack_1` `Action/Stop`)
  (if (`self.Runtime_WeaponReady`)
    (if `Action/Stop`
      (if (> (`self.Runtime_MagazineAmmo`) 0)
        (`self.RepSer_SpawnProjectile` (`SceneComponent.GetSocketTransform` (`self.VisualComponent`) "Muzzle" "RTS_World"))
        (else
          (`KismetSystemLibrary.PrintString` "Reload!!!"))))))

(event `RepSer_SpawnProjectile`
  (params (SpawnTransform :type "Transform Structure"))
  ;[1 1 1] Fire
  (if (> (`self.Runtime_MagazineAmmo`) 0)
    (set `self.Runtime_MagazineAmmo` (- (`self.Runtime_MagazineAmmo`) 1))
    (`|SpawnActorFromClass` (`self.ProjectileClass`) SpawnTransform "AlwaysSpawn" "OverrideRootScale" null null)))

(event `/Game/SurvivalTPSTemp/Blueprints/Player/InventoryComponent/Weapons/Master/BP_SurvTPS_InventoryItem_Weapon_Master.WInput_Attack_2`
  (params (`Action/Stop` :type Boolean))
  (`parent.WInput_Attack_2` `Action/Stop`))

(event `/Game/SurvivalTPSTemp/Blueprints/Player/InventoryComponent/Weapons/Master/BP_SurvTPS_InventoryItem_Weapon_Master.WInput_Reload`
  (params (`Action/Stop` :type Boolean))
  (bind _projectileclass (`self.ProjectileClass`))
  ;[1 1 1] Reload
  (`parent.WInput_Reload` `Action/Stop`)
  (if `Action/Stop`
    (if (`KismetSystemLibrary.IsValidClass` _projectileclass)
      (if (and (> (`/Game/SurvivalTPSTemp/Blueprints/Player/InventoryComponent/BP_SurvTPS_Inventory.GetAmmoTypeAmount` (`/Game/SurvivalTPSTemp/Blueprints/Player/BP_SurvTPS_CharacterMaster.SurvTPS_Inventory` (`self.Runtime_CurrentOwningCharacter`)) (defaults `Object` _projectileclass)) 0) (`self.Runtime_WeaponReady`))
        (`self.RepServ_Reload`)))))

(event `RepServ_Reload`
  ;[1 1 1] Reload
  (set `self.Runtime_WeaponReady` false)
  (`self.RepMulti_Reload`))

(event `RepMulti_Reload`
  ;[1 1 1] Reload
  (`|PlayMontage` (`Character.Mesh` (`self.Runtime_CurrentOwningCharacter`)) (`self.ReloadMontage`)
    (:`OnBlendOut`
      (bind (_newamount _difference) (`/Game/SurvivalTPSTemp/Blueprints/Player/InventoryComponent/BP_SurvTPS_Inventory.ModifyAmmoAmountByType` (`/Game/SurvivalTPSTemp/Blueprints/Player/BP_SurvTPS_CharacterMaster.SurvTPS_Inventory` (`self.Runtime_CurrentOwningCharacter`)) (defaults `Object` (`self.ProjectileClass`)) (- (`self.Runtime_MagazineAmmo`) (`self.MagazineMax`))))
      (set `self.Runtime_MagazineAmmo` (+ (* _difference -1) (`self.Runtime_MagazineAmmo`)))
      (set `self.Runtime_WeaponReady` true))
    (:`OnInterrupted`
      (set `self.Runtime_WeaponReady` true))))

(event `self.ReceiveTick`
  (params (DeltaSeconds :type "Float (single-precision)"))
  (`parent.ReceiveTick` DeltaSeconds))

(event `/Game/SurvivalTPSTemp/Blueprints/Player/InventoryComponent/Weapons/Master/BP_SurvTPS_InventoryItem_Weapon_Master.WInput_Aim`
  (params (`Action/Stop` :type Boolean))
  ;[1 1 1] Comment
  (`parent.WInput_Aim` `Action/Stop`))

(fn `UserConstructionScript`
  (`parent.UserConstructionScript`))