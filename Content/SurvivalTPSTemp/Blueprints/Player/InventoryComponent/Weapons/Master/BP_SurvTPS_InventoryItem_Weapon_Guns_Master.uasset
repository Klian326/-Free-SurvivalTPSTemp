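; Master Blueprint for gun weapon items in the survival TPS inventory, carrying each gun's magazine ammo count inside its item data.
; SetItemData calls the parent, then parses the Runtime_MagazineAmmo additional variable into RuntimeMagazineAmmo, printing an error if it is missing or non-numeric.
; GetItemData writes the current count back into the parent's item struct as a name-encoded additional variable, so ammo travels with the item data.
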(event `self.ReceiveTick`
  (params (DeltaSeconds :type "Float (single-precision)"))
  (`parent.ReceiveTick` DeltaSeconds))

(fn `GetItemData`
  (returns (Struct_SurvTPS_InventoryObject :type "/Game/SurvivalTPSTemp/Blueprints/Player/InventoryComponent/Struct_SurvTPS_InventoryObject Structure"))
  (bind _struct_survtps_inventoryobject (`parent.GetItemData`))
  (bind _structout (`/Game/SurvivalTPSTemp/Blueprints/Player/InventoryComponent/Utility/BPLibrary_SurvTPS_AdditionalVariablesUtility.AddOrEmplace` (`.AdditionalVariables_68_82C693A94807349D0F763FBA7F293858` (break `/Game/SurvivalTPSTemp/Blueprints/Player/InventoryComponent/Struct_SurvTPS_InventoryObject` _struct_survtps_inventoryobject)) "Runtime_MagazineAmmo" (`/Game/SurvivalTPSTemp/Blueprints/Player/InventoryComponent/Utility/BPLibrary_SurvTPS_VariablesTextConversion.IntToName` (`self.Runtime_MagazineAmmo`))))
  (bind _structout_2 (setmembers `/Game/SurvivalTPSTemp/Blueprints/Player/InventoryComponent/Struct_SurvTPS_InventoryObject` :`StructRef` _struct_survtps_inventoryobject :`AdditionalVariables` _structout))
  (return _structout_2))

(fn `SetItemData`
  (params (InData :type "/Game/SurvivalTPSTemp/Blueprints/Player/InventoryComponent/Struct_SurvTPS_InventoryObject Structure"))
  (bind (_value _returnvalue) (`/Game/SurvivalTPSTemp/Blueprints/Player/InventoryComponent/Utility/BPLibrary_SurvTPS_AdditionalVariablesUtility.Find` (`.AdditionalVariables_68_82C693A94807349D0F763FBA7F293858` (break `/Game/SurvivalTPSTemp/Blueprints/Player/InventoryComponent/Struct_SurvTPS_InventoryObject` InData)) "Runtime_MagazineAmmo"))
  (bind (_returnvalue_2 _isvalid) (`/Game/SurvivalTPSTemp/Blueprints/Player/InventoryComponent/Utility/BPLibrary_SurvTPS_VariablesTextConversion.NameToInt` _value))
  (`parent.SetItemData` InData)
  (if _returnvalue
    (if _isvalid
      (set `self.Runtime_MagazineAmmo` _returnvalue_2)
      (return)
      (else
        (`KismetSystemLibrary.PrintString` "Value is not numerical")
        (return)))
    (else
      (`KismetSystemLibrary.PrintString` "Can't find additional variable")
      (return))))

(fn `UserConstructionScript`
  (`parent.UserConstructionScript`))