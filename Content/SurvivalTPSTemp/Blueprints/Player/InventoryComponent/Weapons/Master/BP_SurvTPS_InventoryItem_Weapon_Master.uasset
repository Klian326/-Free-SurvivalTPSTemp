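; Master weapon inventory item for the survival TPS, handling pickup, holstering and dropping, with ready-gated input stubs for child weapons.
; EquipWeapon attaches and assigns ownership, then a multi event snaps the visual to the holster socket without collision.
; UnequipWeapon detaches, sphere-traces down for a surface-aligned drop with random yaw, and restores collision and visual transform.
; ReturnToHolster links unarmed anim layers, reattaches on montage blend-out and clears the equipped weapon on completion.
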(event `self.ReceiveBeginPlay`
  (`parent.ReceiveBeginPlay`)
  (set `self.Runtime_InitialRelativeTransform` (`SceneComponent.GetRelativeTransform` (`self.StaticMesh`))))

(event `RepMulti_ReturnToHolster`
  (params (InSkeletalMeshComponent :type "SkeletalMeshComponent Object Reference"))
  (bind _runtime_currentowningcharacter (`self.Runtime_CurrentOwningCharacter`))
  (`SkeletalMeshComponent.UnlinkAnimClassLayers` InSkeletalMeshComponent "/Game/SurvivalTPSTemp/SkeletalMesh/Characters/Mannequins/Animations/ABP_Layer_Master.ABP_Layer_Master_C")
  (`SkeletalMeshComponent.LinkAnimClassLayers` InSkeletalMeshComponent (`/Game/SurvivalTPSTemp/Blueprints/Player/InventoryComponent/BP_SurvTPS_Inventory.AnimInstanceClassLayerUnarmed` (`/Game/SurvivalTPSTemp/Blueprints/Player/BP_SurvTPS_CharacterMaster.SurvTPS_Inventory` (`self.Runtime_CurrentOwningCharacter`))))
  (`|PlayMontage` InSkeletalMeshComponent (`self.HolsterMontage`)
    (:`OnCompleted`
      (`self.On_IsBackToHolster`)
      (`/Engine/EditorBlueprintResources/StandardMacros.IsValid` _runtime_currentowningcharacter
        (:`Is Valid`
          (set `/Game/SurvivalTPSTemp/Blueprints/Player/InventoryComponent/BP_SurvTPS_Inventory.Runtime_EquippedWeapon` null (`/Game/SurvivalTPSTemp/Blueprints/Player/BP_SurvTPS_CharacterMaster.SurvTPS_Inventory` _runtime_currentowningcharacter)))))
    (:`OnBlendOut`
      (`/Engine/EditorBlueprintResources/StandardMacros.IsValid` (`self.Runtime_CurrentOwningCharacter`)
        (:`Is Valid`
          (`PrimitiveComponent.SetCollisionEnabled` (`self.VisualComponent`) "NoCollision")
          (`SceneComponent.K2_AttachToComponent` (`self.VisualComponent`) InSkeletalMeshComponent (`self.HolsterSocket`) "SnapToTarget" "SnapToTarget" "KeepRelative" false))))
    (:`OnInterrupted`
      (`KismetSystemLibrary.PrintString` "Interrupted"))))

(event `Equip_Multi`
  (params (AttachHolsterComponent :type "SkeletalMeshComponent Object Reference"))
  (`|ExecutionSequence`
    (:`then_0`
      (`/Engine/EditorBlueprintResources/StandardMacros.DoOnce` false
        (:`Completed`
          (set `self.Runtime_DefaultCollisionEnabled` (`PrimitiveComponent.GetCollisionEnabled` (`self.VisualComponent`))))))
    (:`then_1`
      (`PrimitiveComponent.SetCollisionEnabled` (`self.VisualComponent`) "NoCollision")
      (`SceneComponent.K2_AttachToComponent` (`self.VisualComponent`) AttachHolsterComponent (`self.HolsterSocket`) "SnapToTarget" "SnapToTarget" "KeepRelative" false))))

(event `Unequip_Multi`
  (params (NewLocation :type "Vector Structure") (NewRotation :type "Rotator Structure") (`Delta Rotation Z (Yaw)` :type "Float (single-precision)"))
  (`PrimitiveComponent.SetCollisionEnabled` (`self.VisualComponent`) (`self.Runtime_DefaultCollisionEnabled`))
  (`self.K2_SetActorLocationAndRotation` NewLocation NewRotation)
  (`self.K2_AddActorLocalRotation` (`KismetMathLibrary.MakeRotator` 0.0 0.0 `Delta Rotation Z (Yaw)`))
  (`SceneComponent.K2_AttachToComponent` (`self.VisualComponent`) (`self.Root`) "None" "SnapToTarget" "SnapToTarget" "KeepRelative" false)
  (`SceneComponent.K2_SetRelativeTransform` (`self.VisualComponent`) (`self.Runtime_InitialRelativeTransform`) false false))

(event `WInput_Reload`
  (params (`Action/Stop` :type Boolean))
  ;[1 1 1] Will be overwritten in children
  (if (`self.Runtime_WeaponReady`)
    _))

(event `WInput_Attack_1`
  (params (`Action/Stop` :type Boolean))
  ;[1 1 1] Will be overwritten in children
  (if (`self.Runtime_WeaponReady`)
    _))

(event `WInput_Attack_2`
  (params (`Action/Stop` :type Boolean))
  ;[1 1 1] Will be overwritten in children
  (if (`self.Runtime_WeaponReady`)
    _))

(event `WInput_Aim`
  (params (`Action/Stop` :type Boolean))
  ;[1 1 1] Will be overwritten in children
  (if (`self.Runtime_WeaponReady`)
    _))

(fn `EquipWeapon`
  (params (Owner :type "Actor Object Reference"))
  (bind _asbp_surv_tps_character_master (cast `/Game/SurvivalTPSTemp/Blueprints/Player/BP_SurvTPS_CharacterMaster` Owner))
  (bind _output_get (set `self.Runtime_CurrentOwningCharacter` _asbp_surv_tps_character_master))
  (`self.K2_AttachToActor` _output_get "None" "SnapToTarget" "SnapToTarget" "KeepRelative")
  (`self.SetOwner` (`self.Runtime_CurrentOwningCharacter`))
  (`self.Equip_Multi` (`Character.Mesh` (`self.Runtime_CurrentOwningCharacter`)))
  (return))

(fn `ReturnToHolster`
  (params (InputPin :type "Character Object Reference"))
  (returns (Returned :type Boolean))
  (`/Engine/EditorBlueprintResources/StandardMacros.IsValid` InputPin
    (:`Is Valid`
      (`self.RepMulti_ReturnToHolster` (`Character.Mesh` InputPin))
      (return true))
    (:`Is Not Valid`
      (return false))))

(fn `UnequipWeapon`
  (bind _returnvalue (`self.K2_GetActorLocation`))
  (`self.K2_DetachFromActor` "KeepWorld" "KeepWorld" "KeepWorld")
  (`self.SetOwner` null)
  (set `self.Runtime_CurrentOwningCharacter` null)
  (bind (_outhit _returnvalue_2) (`KismetSystemLibrary.SphereTraceSingleForObjects` :`Start` _returnvalue :`End` (- _returnvalue (0.0 0.0 1000.0)) :`Radius` 4.0 :`ObjectTypes` (`|MakeArray` "ObjectTypeQuery1" "ObjectTypeQuery2" :!type "EObjectTypeQuery Enum") :`DrawDebugType` "ForDuration"))
  (if _returnvalue_2
    (bind (_bblockinghit _binitialoverlap _time _distance _location _impactpoint _normal _impactnormal) (`GameplayStatics.BreakHitResult` _outhit))
    (`self.Unequip_Multi` _impactpoint (`KismetMathLibrary.MakeRotFromZ` _impactnormal) (`KismetMathLibrary.RandomFloatInRange` 0.0 360.0))
    (return)
    (else
      (`self.Unequip_Multi` (`self.K2_GetActorLocation`))
      (return))))

(fn `UserConstructionScript`
  (`parent.UserConstructionScript`))