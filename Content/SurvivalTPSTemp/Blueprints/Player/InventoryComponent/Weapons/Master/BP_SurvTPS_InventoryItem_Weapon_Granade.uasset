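; Grenade weapon inventory item for the survival TPS inventory, tracking how many uses remain.
; BeginPlay sets RuntimeUsesLeft to MaxUses.
; GetItemData writes the count into the item's AdditionalVariables as Runtime_UsesLeft, converted to a Name.
; SetItemData reads it back after the parent call, resetting to MaxUses if the entry is missing and leaving it unchanged if invalid.
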(event `self.ReceiveBeginPlay`
  (`parent.ReceiveBeginPlay`)
  (set `self.Runtime_UsesLeft` (`self.MaxUses`)))

(fn `GetItemData`
  (returns (Struct_SurvTPS_InventoryObject :type "/Game/SurvivalTPSTemp/Blueprints/Player/InventoryComponent/Struct_SurvTPS_InventoryObject Structure"))
  (bind _struct_survtps_inventoryobject (`parent.GetItemData`))
  (bind _structout (`/Game/SurvivalTPSTemp/Blueprints/Player/InventoryComponent/Utility/BPLibrary_SurvTPS_AdditionalVariablesUtility.Add` "Runtime_UsesLeft" (`/Game/SurvivalTPSTemp/Blueprints/Player/InventoryComponent/Utility/BPLibrary_SurvTPS_VariablesTextConversion.IntToName` (`self.Runtime_UsesLeft`)) (`.AdditionalVariables_68_82C693A94807349D0F763FBA7F293858` (break `/Game/SurvivalTPSTemp/Blueprints/Player/InventoryComponent/Struct_SurvTPS_InventoryObject` _struct_survtps_inventoryobject))))
  (bind _structout_2 (setmembers `/Game/SurvivalTPSTemp/Blueprints/Player/InventoryComponent/Struct_SurvTPS_InventoryObject` :`StructRef` _struct_survtps_inventoryobject :`AdditionalVariables` _structout))
  (return _structout_2))

(fn `SetItemData`
  (params (InData :type "/Game/SurvivalTPSTemp/Blueprints/Player/InventoryComponent/Struct_SurvTPS_InventoryObject Structure"))
  (bind (_value _returnvalue) (`/Game/SurvivalTPSTemp/Blueprints/Player/InventoryComponent/Utility/BPLibrary_SurvTPS_AdditionalVariablesUtility.Find` (`.AdditionalVariables_68_82C693A94807349D0F763FBA7F293858` (break `/Game/SurvivalTPSTemp/Blueprints/Player/InventoryComponent/Struct_SurvTPS_InventoryObject` InData)) "Runtime_UsesLeft"))
  (bind (_returnvalue_2 _isvalid) (`/Game/SurvivalTPSTemp/Blueprints/Player/InventoryComponent/Utility/BPLibrary_SurvTPS_VariablesTextConversion.NameToInt` _value))
  (`parent.SetItemData` InData)
  (if _returnvalue
    (if _isvalid
      (set `self.Runtime_UsesLeft` _returnvalue_2)
      (return)
      (else
        (return)))
    (else
      (set `self.Runtime_UsesLeft` (`self.MaxUses`))
      (return))))

(fn `UserConstructionScript`
  (`parent.UserConstructionScript`))