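; Survival TPS master HUD that creates and toggles the gameplay, inventory and equipment widgets.
; It caches the pawn's inventory and stats components, updating references on possession change but binding inventory events only at BeginPlay.
; Those events refresh loot, inventory, equipment and ammo displays.
; Loot and inventory views rebuild storage-slot widgets for containers, while loose interacting items fill a shared ground list.
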(event `CreateGameplayUI`
  ;[1 1 1] Create Inventory Widget
  (bind _returnvalue (`|CreateWidget` "/Game/SurvivalTPSTemp/Blueprints/Player/WBP_SurvTPS_GameplayUI.WBP_SurvTPS_GameplayUI_C" (`GameplayStatics.GetPlayerController` 0) self))
  (bind _output_get (set `self.GameplayUI` _returnvalue))
  (`UserWidget.AddToViewport` _output_get 0))

(event `SetGameplayUIVisibility`
  (params (IsVisible :type Boolean))
  ;[1 1 1] Create Inventory Widget
  ;;[1 1 1] Inventory Widget Visibility
  (`Widget.SetVisibility` (`self.GameplayUI`) (select `bool` IsVisible :`false` "Collapsed" :`true` "Visible" :!type "ESlateVisibility Enum")))

(event `self.ReceiveBeginPlay`
  (`|ExecutionSequence`
    (:`then_0`
      (add `Controller.OnPossessedPawnChanged` (`GameplayStatics.GetPlayerController` 0) (delegate `NewPawn`))
      (`self.Refresh Components Refs` (`GameplayStatics.GetPlayerPawn` 0)))
    (:`then_1`
      ;[1 1 1] Refresh loot
      (add `/Game/SurvivalTPSTemp/Blueprints/Player/InventoryComponent/BP_SurvTPS_Inventory.InteractingObjectsChanged` (`self.InventoryComponent`) (delegate `UpdateLoot`)))
    (:`then_2`
      ;[1 1 1] Refresh inventory and loot
      (add `/Game/SurvivalTPSTemp/Blueprints/Player/InventoryComponent/BP_SurvTPS_Inventory.UpdateInventoryUI` (`self.InventoryComponent`) (delegate `UpdateInventoryAndLoot`)))
    (:`then_3`
      (add `/Game/SurvivalTPSTemp/Blueprints/Player/InventoryComponent/BP_SurvTPS_Inventory.RefreshEquipment` (`self.InventoryComponent`) (delegate `RefreshEquipment_Event_0`)))
    (:`then_4`
      (add `/Game/SurvivalTPSTemp/Blueprints/Player/InventoryComponent/BP_SurvTPS_Inventory.RefreshAmmos` (`self.InventoryComponent`) (delegate `RefreshAmmos_Event_0`)))))

(event `NewPawn`
  (params (OldPawn :type "Pawn Object Reference") (NewPawn :type "Pawn Object Reference"))
  (`self.Refresh Components Refs` NewPawn))

(event `CreateInventoryUI`
  ;[1 1 1] Create Inventory Widget
  ;;[1 1 1] Inventory
  (bind _returnvalue (`|CreateWidget` "/Game/SurvivalTPSTemp/Blueprints/Player/InventoryComponent/UI/Inventory/WBP_SurvTPS_InventoryUI.WBP_SurvTPS_InventoryUI_C" (`GameplayStatics.GetPlayerController` 0) self))
  (bind _output_get (set `self.InventoryUI` _returnvalue))
  (`UserWidget.AddToViewport` _output_get 0)
  (`self.RefreshLootWidget`))

(event `SetInventoryWidgetVisibility`
  (params (IsVisible :type Boolean))
  ;[1 1 1] Create Inventory Widget
  ;;[1 1 1] Inventory
  ;;;[1 1 1] Inventory Widget Visibility
  (`Widget.SetVisibility` (`self.InventoryUI`) (select `bool` IsVisible :`false` "Collapsed" :`true` "Visible" :!type "ESlateVisibility Enum")))

(event `CreateEquipmentUI`
  ;[1 1 1] Create Inventory Widget
  ;;[1 1 1] Equipment
  (bind _returnvalue (`|CreateWidget` "/Game/SurvivalTPSTemp/Blueprints/Player/InventoryComponent/UI/Equipment/WBP_SurvTPS_EquipmentUI.WBP_SurvTPS_EquipmentUI_C" (`GameplayStatics.GetPlayerController` 0) self))
  (bind _output_get (set `self.EquipmentUI` _returnvalue))
  (`UserWidget.AddToViewport` _output_get 0))

(event `UpdateLoot`
  ;[1 1 1] Refresh loot
  (`self.RefreshLootWidget`))

(event `SetEquipmentWidgetVisibility`
  (params (IsVisible :type Boolean))
  ;[1 1 1] Create Inventory Widget
  ;;[1 1 1] Equipment
  ;;;[1 1 1] Inventory Widget Visibility
  (`Widget.SetVisibility` (`self.EquipmentUI`) (select `bool` IsVisible :`false` "Collapsed" :`true` "Visible" :!type "ESlateVisibility Enum")))

(event `UpdateInventoryAndLoot`
  ;[1 1 1] Refresh inventory and loot
  (`self.RefreshInventoryWidget`)
  (`self.RefreshLootWidget`)
  (`self.RefreshAllContainers`))

(event `RefreshEquipment_Event_0`
  (`/Game/SurvivalTPSTemp/Blueprints/Player/InventoryComponent/UI/Equipment/WBP_SurvTPS_EquipSlots.RefreshAllEquip` (`/Game/SurvivalTPSTemp/Blueprints/Player/InventoryComponent/UI/Equipment/WBP_SurvTPS_EquipmentUI.W_EquipSlots` (`self.EquipmentUI`))))

(event `RefreshAmmos_Event_0`
  (`/Game/SurvivalTPSTemp/Blueprints/Player/InventoryComponent/UI/Equipment/WBP_SurvTPS_EquipSlots.RefreshAllAmmo` (`/Game/SurvivalTPSTemp/Blueprints/Player/InventoryComponent/UI/Equipment/WBP_SurvTPS_EquipmentUI.W_EquipSlots` (`self.EquipmentUI`))))

(fn `AddStorageSlotWidgetWithContainedItems`
  (params (SlotsList :type "/Game/SurvivalTPSTemp/Blueprints/Player/InventoryComponent/UI/Inventory/WBP_SurvTPS_SlotsList Object Reference") (ContainerItem :type "/Game/SurvivalTPSTemp/Blueprints/Player/InventoryComponent/BP_SurvTPS_InventoryItem_Master Object Reference") (ContainedItems :type "Array of /Game/SurvivalTPSTemp/Blueprints/Player/InventoryComponent/Struct_SurvTPS_InventoryObject Structure") (SlotsReferenceList :type "Array of /Game/SurvivalTPSTemp/Blueprints/Player/InventoryComponent/UI/Inventory/WBP_SurvTPS_StorageSlot Object Reference (by ref)"))
  (bind _returnvalue (`|CreateWidget` "/Game/SurvivalTPSTemp/Blueprints/Player/InventoryComponent/UI/Inventory/WBP_SurvTPS_StorageSlot.WBP_SurvTPS_StorageSlot_C" (`GameplayStatics.GetPlayerController` 0) self (`/Game/SurvivalTPSTemp/Blueprints/Player/InventoryComponent/BP_SurvTPS_InventoryItem_Master.GetItemData` ContainerItem) ContainedItems null))
  (`KismetArrayLibrary.Array_Add` SlotsReferenceList _returnvalue)
  (`PanelWidget.AddChild` (`/Game/SurvivalTPSTemp/Blueprints/Player/InventoryComponent/UI/Inventory/WBP_SurvTPS_SlotsList.W_HorizontalScrollBox` SlotsList) _returnvalue)
  (`/Game/SurvivalTPSTemp/Blueprints/Player/InventoryComponent/UI/Inventory/WBP_SurvTPS_StorageSlot.Update Slot Title and Capacity` _returnvalue "None")
  (return))

(fn `ClearContainers`
  (params (Array :type "Array of /Game/SurvivalTPSTemp/Blueprints/Player/InventoryComponent/UI/Inventory/WBP_SurvTPS_StorageSlot Object Reference"))
  (for _array_element Array
    (`/Engine/EditorBlueprintResources/StandardMacros.IsValid` _array_element
      (:`Is Valid`
        (`Widget.RemoveFromParent` _array_element))))
  (`KismetArrayLibrary.Array_Clear` Array)
  (return))

(fn `Refresh Components Refs`
  (params (NewPawn :type "Pawn Object Reference"))
  (`/Engine/EditorBlueprintResources/StandardMacros.IsValid` NewPawn
    (:`Is Valid`
      (set `self.InventoryComponent` (`self.GetComponentByClass` NewPawn "/Game/SurvivalTPSTemp/Blueprints/Player/InventoryComponent/BP_SurvTPS_Inventory.BP_SurvTPS_Inventory_C"))
      (set `self.StatsComponent` (`self.GetComponentByClass` NewPawn "/Game/SurvivalTPSTemp/Blueprints/Player/SurvivalComponent/BP_SurvTPS_Stats.BP_SurvTPS_Stats_C"))
      (return))
    (:`Is Not Valid`
      (set `self.InventoryComponent` null)
      (set `self.StatsComponent` null)
      (return))))

(fn `RefreshAllContainers`
  (locals (L_WidgetsToRefresh :type "Array of /Game/SurvivalTPSTemp/Blueprints/Player/InventoryComponent/UI/Inventory/WBP_SurvTPS_StorageSlot Object Reference"))
  (bind _output_get (set `local.L_WidgetsToRefresh` (`self.ContainersGroundWidgets`)))
  (`KismetArrayLibrary.Array_Append` _output_get (`self.ContainersInventoryWidgets`))
  (for _array_element (`local.L_WidgetsToRefresh`)
    (`/Game/SurvivalTPSTemp/Blueprints/Player/InventoryComponent/UI/Inventory/WBP_SurvTPS_StorageSlot.Update Slot Title and Capacity` _array_element "None")))

(fn `RefreshInventoryWidget`
  (bind _inventorycomponent (`self.InventoryComponent`))
  (`self.ClearContainers` (`self.ContainersInventoryWidgets`))
  (`/Engine/EditorBlueprintResources/StandardMacros.IsValid` _inventorycomponent
    (:`Is Valid`
      (for _array_element (`/Game/SurvivalTPSTemp/Blueprints/Player/InventoryComponent/BP_SurvTPS_Inventory.Equipment` _inventorycomponent)
        (`/Engine/EditorBlueprintResources/StandardMacros.IsValid` _array_element
          (:`Is Valid`
            (if (> (`/Game/SurvivalTPSTemp/Blueprints/Player/InventoryComponent/BP_SurvTPS_InventoryItem_Master.StorageVolumeMax` _array_element) 0.0)
              (`self.AddStorageSlotWidgetWithContainedItems` (`/Game/SurvivalTPSTemp/Blueprints/Player/InventoryComponent/UI/Inventory/WBP_SurvTPS_InventoryUI.Wc_InventorySlotsList` (`self.InventoryUI`)) _array_element (`/Game/SurvivalTPSTemp/Blueprints/Player/InventoryComponent/BP_SurvTPS_InventoryItem_Master.Runtime_StoredItems` _array_element) (`self.ContainersInventoryWidgets`))))))
      (return))))

(fn `RefreshLootWidget`
  (locals (L_ItemRef :type "/Game/SurvivalTPSTemp/Blueprints/Player/InventoryComponent/BP_SurvTPS_InventoryItem_Master Object Reference"))
  (bind _runtime_storeditems (`/Game/SurvivalTPSTemp/Blueprints/Player/InventoryComponent/BP_SurvTPS_InventoryItem_Master.Runtime_StoredItems` (`local.L_ItemRef`)))
  (`/Game/SurvivalTPSTemp/Blueprints/Player/InventoryComponent/UI/Inventory/WBP_SurvTPS_StorageSlot.ClearList` (`/Game/SurvivalTPSTemp/Blueprints/Player/InventoryComponent/UI/Inventory/WBP_SurvTPS_InventoryUI.Wcc_StorageSlot_Ground` (`self.InventoryUI`)))
  (`self.ClearContainers` (`self.ContainersGroundWidgets`))
  (`/Engine/EditorBlueprintResources/StandardMacros.IsValid` (`self.InventoryComponent`)
    (:`Is Valid`
      (for _array_element (`/Game/SurvivalTPSTemp/Blueprints/Player/InventoryComponent/BP_SurvTPS_Inventory.Runtime_InteractingActors` (`self.InventoryComponent`))
        (`/Engine/EditorBlueprintResources/StandardMacros.IsValid` _array_element
          (:`Is Valid`
            (bind _output_get (set `local.L_ItemRef` _array_element))
            (`/Engine/EditorBlueprintResources/StandardMacros.IsValid` _output_get
              (:`Is Valid`
                (if (or (> (`KismetArrayLibrary.Array_Length` _runtime_storeditems) 0) (> (`/Game/SurvivalTPSTemp/Blueprints/Player/InventoryComponent/BP_SurvTPS_InventoryItem_Master.StorageVolumeMax` _output_get) 0.0))
                  (`self.AddStorageSlotWidgetWithContainedItems` (`/Game/SurvivalTPSTemp/Blueprints/Player/InventoryComponent/UI/Inventory/WBP_SurvTPS_InventoryUI.Wc_LootSlotsList` (`self.InventoryUI`)) (`local.L_ItemRef`) _runtime_storeditems (`self.ContainersGroundWidgets`))
                  (else
                    (`/Game/SurvivalTPSTemp/Blueprints/Player/InventoryComponent/UI/Inventory/WBP_SurvTPS_StorageSlot.AddItemToList` (`/Game/SurvivalTPSTemp/Blueprints/Player/InventoryComponent/UI/Inventory/WBP_SurvTPS_InventoryUI.Wcc_StorageSlot_Ground` (`self.InventoryUI`)) (`/Game/SurvivalTPSTemp/Blueprints/Player/InventoryComponent/BP_SurvTPS_InventoryItem_Master.GetItemData` _array_element) null 0 :!label _label))))
              (:`Is Not Valid`
                (goto _label))))))
      (return))
    (:`Is Not Valid`
      (return))))

(fn `ShowAimSign`
  (params (Index :type Boolean))
  (`/Game/SurvivalTPSTemp/Blueprints/Player/WBP_SurvTPS_GameplayUI.SetAimSignVisibility` (`self.GameplayUI`) Index))

(fn `UserConstructionScript`)