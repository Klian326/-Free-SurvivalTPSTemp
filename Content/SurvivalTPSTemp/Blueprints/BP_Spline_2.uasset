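; Spline placement Blueprint that lines a path with repeated static meshes, built entirely in the Construction Script.
; Each rebuild clears the old components, then adds rigid Static Mesh Components at steps of mesh length plus Spacing, with the count derived from spline and mesh length alone.
; Each piece is rotated toward the next point rather than deformed, wrapping to the start when CloseLoop is set.
; MeshVariants can override the default mesh by index.
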(fn `UserConstructionScript`
  (locals (SectionLength :type "Float (double-precision)"))
  (bind _staticmeshvar (`self.StaticMeshVar`))
  (bind _returnvalue (`KismetMathLibrary.FTrunc` (/ (`SplineComponent.GetSplineLength` (`self.Spline`)) (`local.SectionLength`))))
  (`/Engine/EditorBlueprintResources/StandardMacros.IsValid` _staticmeshvar
    (:`Is Valid`
      (set `local.SectionLength` (* 2 (.x (`.BoxExtent` (`KismetMathLibrary.BreakBoxSphereBounds` (`StaticMesh.GetBounds` _staticmeshvar))))))
      (`SplineComponent.SetClosedLoop` (`self.Spline`) (`self.CloseLoop`) true)
      (for _array_element (`self.SplineMeshes`)
        (`ActorComponent.K2_DestroyComponent` _array_element))
      (`KismetArrayLibrary.Array_Clear` (`self.SplineMeshes`))
      (for _index (range (+ (- _returnvalue (`KismetMathLibrary.SelectInt` 0 1 (`self.CloseLoop`))) 1))
        (bind _returnvalue_2 (`SplineComponent.GetLocationAtDistanceAlongSpline` (`self.Spline`) (+ (* _index (`self.Spacing`)) (* _index (`local.SectionLength`))) "Local"))
        (bind _returnvalue_3 (`KismetMathLibrary.SelectInt` 0 (+ _index 1) (and (== _index _returnvalue) (`self.CloseLoop`))))
        (bind _returnvalue_4 (`AddComponent|NODE_AddStaticMeshComponent-0` :`RelativeTransform` (`KismetMathLibrary.MakeTransform` (+ _returnvalue_2 (0.0 0.0 0.0)) (`KismetMathLibrary.FindLookAtRotation` _returnvalue_2 (`SplineComponent.GetLocationAtDistanceAlongSpline` (`self.Spline`) (+ (* _returnvalue_3 (`local.SectionLength`)) (* _returnvalue_3 (`self.Spacing`))) "Local")))))
        (`KismetArrayLibrary.Array_Add` (`self.SplineMeshes`) _returnvalue_4)
        (`StaticMeshComponent.SetStaticMesh` _returnvalue_4 (select `bool` (`BlueprintMapLibrary.Map_Contains` (`self.MeshVariants`) _index) :`false` (`self.StaticMeshVar`) :`true` (`BlueprintMapLibrary.Map_Find` (`self.MeshVariants`) _index)))))))